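; BP_EnemyBase is a base enemy that periodically fires anti-player projectiles and can be knocked back when hit.
; A Delay on Tick paces the shots a few seconds apart.
; Each shot leads the target, using distance over projectile speed to request the player's predicted position, then spawns a projectile aimed there from the spawn point.
; GetHit launches the character along the given direction, scaled by magnitude.
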(event `self.ReceiveBeginPlay`)

(event `self.ReceiveTick`
  (params (DeltaSeconds :type "Float (single-precision)"))
  (`KismetSystemLibrary.Delay` 4.0)
  (`self.LaunchProjectileAtPlayer`))

(event `/Game/enemies/BPI_EnemyInterface.GetHit`
  (params (Direction :type "Vector Structure") (Magnitude :type "Float (double-precision)"))
  (`self.LaunchCharacter` (* Direction Magnitude)))

(fn `GetDistanceFromPlayer`
  (returns (`Distance From Player` :type "Float (double-precision)"))
  (return (`KismetMathLibrary.Vector_Distance` (`self.K2_GetActorLocation`) (`self.K2_GetActorLocation` (`/Game/GameEssentials/CommonFunctionLibrary.GetMyPlayerCharacter`)))))

(fn `LaunchProjectileAtPlayer`
  (bind _projectilespeed (`self.ProjectileSpeed`))
  (bind _projectilespawnpoint (`self.ProjectileSpawnPoint`))
  ; Where to Launch
  (bind _returnvalue (`/Game/FirstPerson/Blueprints/BP_FirstPersonCharacter.PlayerFuturePosition` (`/Game/GameEssentials/CommonFunctionLibrary.GetMyPlayerCharacter`) (/ (`self.GetDistanceFromPlayer`) (`self.ProjectileSpeed`))))
  (`|SpawnActorFromClass` "/Game/FirstPerson/Projectiles/BP_AntiPlayerProjectileBase.BP_AntiPlayerProjectileBase_C" (`KismetAnimationLibrary.K2_LookAt` (`SceneComponent.K2_GetComponentToWorld` _projectilespawnpoint) _returnvalue (`SceneComponent.GetForwardVector` _projectilespawnpoint)) "Undefined" "MultiplyWithRoot" null 5.0 _projectilespeed _projectilespeed true self))

(fn `UserConstructionScript`)